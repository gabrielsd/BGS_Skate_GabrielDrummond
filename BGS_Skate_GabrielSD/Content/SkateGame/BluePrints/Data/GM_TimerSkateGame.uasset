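; Game mode for the skate game that runs a countdown and ends play when time runs out.
; BeginPlay creates the W_MainGameplay widget, sets game-only input and starts a looping one-second timer that decrements Timer.
; At zero, it slows global time to near-freeze, disables player input, shows the cursor, switches the widget to another panel and sets UI-only input.
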(event Custom|DecreaseTimer
  (bind _widget_ref (Variables|Default|GetWidget_Ref))
  (if (<= (Variables|Default|GetTimer) 0.0)
    (Utilities|Time|SetGlobalTimeDilation 0.05)
    (Input|DisableInput (Game|GetPlayerCharacter 0) 0)
    (Variables|/Script/Engine.PlayerController|SetbShowMouseCursor (Game|GetPlayerController 0) true)
    (Default|ChangeSwitcherIndex _widget_ref 3)
    (Input|SetInputModeUIOnly (Game|GetPlayerController 0) _widget_ref "DoNotLock" false)
    (else
      (Variables|Default|SetTimer (- (Variables|Default|GetTimer) 1.0)))))

(event EventBeginPlay
  (Utilities|Time|SetTimerbyEvent (delegate Custom|DecreaseTimer) 1.0 true)
  (bind _returnvalue (UserInterface|CreateWidget "/Game/SkateGame/BluePrints/Widget/W_MainGameplay.W_MainGameplay_C"))
  (bind _output_get (Variables|Default|SetWidget_Ref _returnvalue))
  (UserInterface|Viewport|AddtoViewport _output_get 0)
  (Input|SetInputModeGameOnly (Game|GetPlayerController 0) false))

(event EventTick
  (params (DeltaSeconds :type Float%20%28single-precision%29)))

(fn ConstructionScript)