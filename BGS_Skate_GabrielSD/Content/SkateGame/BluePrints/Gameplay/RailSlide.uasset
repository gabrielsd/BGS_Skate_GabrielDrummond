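; Rail actor the player can slide along when falling onto it roughly aligned with its direction, earning points for the ride.
; Overlapping the box passes a DoOnce, attaches the pawn to PlayerAttach and picks direction from facing.
; A looping timer moves PlayerAttach along a two-point spline.
; At either end it detaches and launches the player, re-arms, plays a sound and awards points scaled by distance slid.
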(event OnComponentBeginOverlap(Box)
  (params (OverlappedComponent :type Primitive%20Component%20Object%20Reference) (OtherActor :type Actor%20Object%20Reference) (OtherComp :type Primitive%20Component%20Object%20Reference) (OtherBodyIndex :type Integer) (bFromSweep :type Boolean) (SweepResult :type Hit%20Result%20Structure%20%28by%20ref%29))
  (bind _returnvalue (Transformation|GetActorForwardVector))
  (bind _returnvalue_2 (Game|Player|GetPlayerPawn 0))
  (bind _returnvalue_3 (Game|Player|GetPlayerPawn 0))
  (bind _returnvalue_4 (Transformation|GetActorForwardVector _returnvalue_2))
  (bind _returnvalue_5 (Math|Vector|DotProduct _returnvalue_4 _returnvalue))
  (if (== OtherActor _returnvalue_2)
    (if (and (> (Math|Float|Absolute(Float) _returnvalue_5) 0.6) (AI|Components|NavMovement|IsFalling (Variables|/Script/Engine.Character|GetCharacterMovement (Game|GetPlayerCharacter 0))))
      (Utilities|FlowControl|DoOnce false
        (:Completed
          (bind _output_get (Variables|Default|SetStartingDotProduct _returnvalue_5))
          (Variables|Default|SetDirectionRight? (> _output_get 0.0))
          (bind _output_get_2 (Variables|Default|SetPlayerCurrentPositionInSpline (Class|SplineComponent|GetDistanceAlongSplineatLocation (Variables|Default|GetSpline) (Transformation|GetActorLocation (Game|Player|GetPlayerPawn 0)) "World")))
          (Variables|Default|SetPlayer%20Start%20Position _output_get_2)
          (Class|BPISkatePlayerInterface|StartSlide(Message) _returnvalue_3)
          (Transformation|AttachComponentToComponent _returnvalue_3 (Variables|Default|GetPlayerAttach) "None" "SnapToTarget" "KeepWorld" "KeepWorld" true)
          (Utilities|Time|SetTimerbyFunctionName 0 "UpdatePlayerLocationOnRail" 0.005 true))))))

(event Custom|UpdatePlayerLocationOnRail
  (bind _returnvalue (Game|Player|GetPlayerPawn 0))
  (bind _sliderate (Variables|Default|GetSlideRate))
  (bind _playerattach (Variables|Default|GetPlayerAttach))
  (bind _returnvalue_2 (Math|Vector|GetForwardVector _playerattach))
  (Transformation|SetRelativeLocation (Variables|Default|GetPlayerAttach) (+ (Spline|GetLocationatDistanceAlongSpline (Variables|Default|GetSpline) (Variables|Default|GetPlayerCurrentPositionInSpline) "Local") (Variables|Default|GetPlayerOffset)) true true)
  (bind _output_get (Variables|Default|SetPlayerCurrentPositionInSpline (Math|Float|Clamp(Float) (+ (Variables|Default|GetPlayerCurrentPositionInSpline) (Math|Float|SelectFloat (* _sliderate -1.0) _sliderate (Variables|Default|GetDirectionRight?))) 0.0 (Spline|GetSplineLength (Variables|Default|GetSpline)))))
  (if (or (== _output_get 0.0) (== _output_get (Spline|GetSplineLength (Variables|Default|GetSpline))))
    (Utilities|Time|ClearTimerbyFunctionName 0 "UpdatePlayerLocationOnRail")
    (Class|BPISkatePlayerInterface|StopSlide(Message) _returnvalue)
    (Transformation|DetachFromActor _returnvalue "KeepWorld" "KeepWorld" "KeepWorld")
    (Character|LaunchCharacter (Game|GetPlayerCharacter 0) (+ (* (Math|Vector|SelectVector _returnvalue_2 (* _returnvalue_2 -1) (Variables|Default|GetDirectionRight?)) 1000) "0.000000,0.000000,400.000000") true true)
    (CallFunction|SliderReset)
    (Class|BPISkatePlayerInterface|CollectPoints(Message) (Game|GetPlayerCharacter 0) (Math|Float|Truncate (Math|Float|SelectFloat (Math|Float|MapRangeClamped (Variables|Default|GetPlayer%20Start%20Position) 0.0 (Spline|GetSplineLength (Variables|Default|GetSpline)) 1e+02 6e+02) (Math|Float|MapRangeClamped (Variables|Default|GetPlayer%20Start%20Position) (Spline|GetSplineLength (Variables|Default|GetSpline)) 0.0 1e+02 6e+02) (Variables|Default|GetDirectionRight?))))
    (Audio|PlaySound2D "/Game/Interface_And_Item_Sounds/Cues/Futuristic_Click_02_Cue.Futuristic_Click_02_Cue" 1.1 1.3 0.0 0 0)))

(event Custom|SliderReset
  (bind _returnvalue (Game|Player|GetPlayerPawn 0))
  (Utilities|FlowControl|DoOnce false) ; enters at Reset
)

(event EventBeginPlay
  ;[1 1 1] Setup Spline
  (Spline|SetLocationatSplinePoint (Variables|Default|GetSpline) 0 (Variables|Default|GetStartLocation) "Local" true)
  (Spline|SetLocationatSplinePoint (Variables|Default|GetSpline) 1 (Variables|Default|GetEndLocation) "Local" true))

(event Collision|EventActorBeginOverlap
  (params (OtherActor :type Actor%20Object%20Reference)))

(event EventTick
  (params (DeltaSeconds :type Float%20%28single-precision%29)))

(fn ConstructionScript)