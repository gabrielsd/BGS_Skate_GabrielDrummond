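; GridSpawner is an editor-placed tool actor that lays out copies of one static mesh in a two-dimensional grid.
; Its construction script runs nested loops over XAmount and YAmount, adding a static mesh component at each cell, spaced by XDistance and YDistance.
; IsVertical switches the second axis from Y to Z, turning a flat grid into an upright one.
; The event graph holds no logic.
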(event EventBeginPlay)

(event Collision|EventActorBeginOverlap
  (params (OtherActor :type Actor%20Object%20Reference)))

(event EventTick
  (params (DeltaSeconds :type Float%20%28single-precision%29)))

(fn ConstructionScript
  (Utilities|IsValid (Variables|Default|GetStaticMeshRef)
    (:Is%20Valid
      (for _index (range 0 (Variables|Default|GetXAmount))
        (for _index_2 (range 0 (Variables|Default|GetYAmount))
          (bind _returnvalue (AddComponent|AddStaticMeshComponent false (Math|Transform|MakeTransform (Math|Vector|MakeVector (* _index (Variables|Default|GetXDistance)) (Math|Float|SelectFloat 0.0 (* _index_2 (Variables|Default|GetYDistance)) (Variables|Default|GetIsVertical?)) (Math|Float|SelectFloat (* _index_2 (Variables|Default|GetYDistance)) 0.0 (Variables|Default|GetIsVertical?))) "0, 0, 0" "1.000000,1.000000,1.000000")))
          (Components|StaticMesh|SetStaticMesh _returnvalue (Variables|Default|GetStaticMeshRef)))))))