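; BP_SplineCollectableSpawner is a tool actor that places copies of a chosen actor class, by its name collectables, at even intervals along a spline.
; SpawnAlongSpline divides the spline length by SpawnDistance and spawns ActorToSpawn at each step.
; It adds local spline points to the actor's location, so actor rotation and scale are ignored.
; Both the construction script and BeginPlay call it, with no cleanup of earlier spawns.
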(event EventBeginPlay
  (CallFunction|SpawnAlongSpline))

(event Collision|EventActorBeginOverlap
  (params (OtherActor :type Actor%20Object%20Reference)))

(event EventTick
  (params (DeltaSeconds :type Float%20%28single-precision%29)))

(fn ConstructionScript
  (CallFunction|SpawnAlongSpline))

(fn SpawnAlongSpline
  (for _index (range 0 (Math|Float|Truncate (/ (Spline|GetSplineLength (Variables|Default|GetSpline)) (Variables|Default|GetSpawnDistance))))
    (Game|SpawnActorfromClass (Variables|Default|GetActorToSpawn) (Math|Transform|MakeTransform (+ (Spline|GetLocationatDistanceAlongSpline (Variables|Default|GetSpline) (* _index (Variables|Default|GetSpawnDistance)) "Local") (Transformation|GetActorLocation)) "0, 0, 0" "1.000000,1.000000,1.000000") "Undefined" "MultiplyWithRoot" 0 0)))